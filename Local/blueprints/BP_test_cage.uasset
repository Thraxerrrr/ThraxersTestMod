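; BP_test_cage is a test cage actor that places a character on itself in a sitting pose when activated.
; On interaction, it casts the instigator's pawn to BaseBPChar, teleports it above the interactable component and starts the SitOnGround emote through the EmoteController.
; Collision toggling and delayed binding to character movement are left unconnected, and the movement handler is empty.
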(event `self.InteractableActivate`
  (params (Component :type "PrimitiveComponent Object Reference") (Instigator :type "PlayerController Object Reference") (HitIndex :type Integer) (TriggeredFromRadialWheel :type Boolean))
  (bind _asbase_bpchar (cast `/Game/Characters/BaseBPChar` (`Controller.K2_GetPawn` Instigator)))
  (`self.K2_SetActorLocation` _asbase_bpchar (+ (`SceneComponent.K2_GetComponentLocation` Component) (0.0 0.0 150.0)) false true)
  (`EmoteController.StartEmote` (`ConanCharacter.EmoteController` _asbase_bpchar) "SitOnGround"))

(event `OnCharMove`
  (params (DeltaSeconds :type "Float (double-precision)") (OldLocation :type "Vector Structure") (OldVelocity :type "Vector Structure")))

(fn `UserConstructionScript`
  (`parent.UserConstructionScript`))