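; BP_lantern_short is a lantern Blueprint with unwired logic for hanging a static mesh on the player character's right thigh socket.
; The attach chain creates a component tagged LanternIsAttached, or reuses the tagged one, though SetStaticMesh is given no mesh.
; A separate chain detaches that tagged component.
; Neither chain is connected to an event, and BeginPlay only calls its parent, so none of this logic runs.
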(event `self.ReceiveBeginPlay`
  (`parent.ReceiveBeginPlay`))

(event `self.ReceiveEndPlay`
  (params (EndPlayReason :type "EEndPlayReason Enum" :default "Destroyed")))

(fn `UserConstructionScript`
  (`parent.UserConstructionScript`))