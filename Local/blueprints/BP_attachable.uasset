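; BP_attachable is a usable item that toggles an attachment on the character who uses it.
; On use, it destroys the attached actor if present; otherwise the server spawns one and snaps it to a target socket on the character's mesh.
; The spawned actor is a BP_attaching_actor carrying MeshToAttach when that mesh is valid, or an instance of the ActorToAttach class as fallback.
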(event `self.OnUseItem`
  (params (invokingCharacter :type "ConanCharacter Object Reference"))
  (`self.ToggleAttach` invokingCharacter))

(fn `CanUseItem`
  (params (invokingCharacter :type "ConanCharacter Object Reference"))
  (returns (ReturnValue :type Boolean))
  (return true))

(fn `ToggleAttach`
  (params (TargetCharacter :type "ConanCharacter Object Reference"))
  (bind _meshtoattach (`self.MeshToAttach`))
  (set `self.ParentCharacter` TargetCharacter)
  (if (`self.IsMeshAttached`)
    (`Actor.K2_DestroyActor` (`self.AttachedActor`))
    (set `self.IsMeshAttached` false)
    (elif (`KismetSystemLibrary.IsServer`)
      (bind _worldcomponenttransform (`CharacterFunctionLibrary.GetWorldComponentTransform` (`Character.Mesh` (`self.ParentCharacter`))))
      (`/Game/Systems/BP_MacroGlobal.IsValid+Branch` _meshtoattach true
        (:`True`
          (bind _returnvalue (`|SpawnActorFromClass` "/Game/Mods/ThraxersTestMod/blueprints/BP_attaching_actor.BP_attaching_actor_C" _worldcomponenttransform "Undefined" "OverrideRootScale"))
          (`StaticMeshComponent.SetStaticMesh` (`/Game/Mods/ThraxersTestMod/blueprints/BP_attaching_actor.StaticMesh` _returnvalue) (`self.MeshToAttach`)))
        (:`False or Invalid`
          (bind _returnvalue_2 (`|SpawnActorFromClass` (`self.ActorToAttach`) _worldcomponenttransform "Undefined" "OverrideRootScale"))))
      (bind _asactor (cast `Actor` (`KismetMathLibrary.SelectObject` _returnvalue _returnvalue_2 (`KismetSystemLibrary.IsValid` _meshtoattach))))
      (bind _output_get (set `self.AttachedActor` _asactor))
      (`Actor.K2_AttachToComponent` _output_get (`Character.Mesh` (`self.ParentCharacter`)) (`self.TargetSocket`) "SnapToTarget" "SnapToTarget" "SnapToTarget" true)
      (set `self.IsMeshAttached` true))))