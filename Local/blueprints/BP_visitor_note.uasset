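; BP_visitor_note is a placeable note actor that the player can remove through its interaction radial menu.
; The menu gets a Remove entry, which sends a dismantle message for the note through the first player's character.
; CanBePlaced defers to the parent check but turns its vertical-surface failure into a success by matching the error text, so the note is not limited to vertical surfaces.
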(event `/Game/Systems/Building/Placeables/BP_Master_Placeables.InteractableMenu`
  (params (RadialMenu :type "RadialMenu Object Reference") (HitIndex :type Integer))
  (bind _returnvalue (`RadialMenu.AddItem` RadialMenu "Remove" "Remove this note" "/Game/UI/Textures/GUIs/MainRadialMenu/T_MainRadialMenuIconDismantle.T_MainRadialMenuIconDismantle" "None" 0))
  (add `RadialMenuEntry.SignalClicked` _returnvalue (delegate `OnRemoveClicked`)))

(event `OnRemoveClicked`
  (params (menuEntry :type "RadialMenuEntry Object Reference"))
  (message `/Game/Systems/Interfaces/BasePlayerCharInterface.Player Interactable Dismantle` (`GameplayStatics.GetPlayerCharacter` 0) self))

(fn `CanBePlaced`
  (params (AttachTo :type "BuildableBase Object Reference") (InstanceIndex :type Integer))
  (returns (FailedMessage :type String) (ReturnValue :type "ECanBePlacedResult Enum"))
  (bind (_failedmessage _returnvalue) (`parent.CanBePlaced` null 0))
  (if (`KismetStringLibrary.EqualEqual_StrStr` _failedmessage "Must be attached to a vertical enough surface")
    (return "" "Success")
    (else
      (return _failedmessage _returnvalue))))

(fn `UserConstructionScript`
  (`parent.UserConstructionScript`))