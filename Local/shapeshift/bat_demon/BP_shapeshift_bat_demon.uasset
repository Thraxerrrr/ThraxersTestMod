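; Usable item that shapeshifts the using character into a bat demon through BP_shapeshift_bat_demon_comp.
; A 0.3-second timer separates single from double use: a second use cancels it and calls ToggleForm(true) on the stored component.
; When the timer expires, the server adds the skeletal mesh component if the character lacks one, then calls ToggleForm(false).
; The double-use path neither creates the component nor checks for server authority.
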(event `ExecOnUse`
  (`KismetSystemLibrary.K2_ClearAndInvalidateTimerHandle` (`self.DelayedExecTimer`))
  (if (`KismetSystemLibrary.IsServer`)
    (`|ExecutionSequence`
      (:`then_0`
        (`/Game/Systems/BP_MacroGlobal.IsValid+Branch` (`Actor.GetComponentByClass` (`self.TargetCharacter`) "/Game/Mods/ThraxersTestMod/shapeshift/bat_demon/BP_shapeshift_bat_demon_comp.BP_shapeshift_bat_demon_comp_C") true
          (:`False or Invalid`
            (bind _returnvalue (`CharacterFunctionLibrary.AddSkeletalMeshComponent` (`self.TargetCharacter`) false (`KismetMathLibrary.Conv_VectorToTransform` (0.0 0.0 0.0)) "/Game/Mods/ThraxersTestMod/shapeshift/bat_demon/BP_shapeshift_bat_demon_comp.BP_shapeshift_bat_demon_comp_C"))
            (bind _asbp_shapeshift_bat_demon_comp (cast `/Game/Mods/ThraxersTestMod/shapeshift/bat_demon/BP_shapeshift_bat_demon_comp` _returnvalue))
            (set `self.ShapeshiftComponent` _asbp_shapeshift_bat_demon_comp))))
      (:`then_1`
        (`/Game/Mods/ThraxersTestMod/shapeshift/bat_demon/BP_shapeshift_bat_demon_comp.ToggleForm` (`self.ShapeshiftComponent`) false)))))

(event `self.OnUseItem`
  (params (invokingCharacter :type "ConanCharacter Object Reference"))
  (bind _delayedexectimer (`self.DelayedExecTimer`))
  (bind _asbase_bpchar (cast `/Game/Characters/BaseBPChar` invokingCharacter))
  (set `self.TargetCharacter` _asbase_bpchar)
  (if (`KismetSystemLibrary.K2_IsValidTimerHandle` _delayedexectimer)
    (`KismetSystemLibrary.K2_ClearAndInvalidateTimerHandle` _delayedexectimer)
    (`/Game/Mods/ThraxersTestMod/shapeshift/bat_demon/BP_shapeshift_bat_demon_comp.ToggleForm` (`self.ShapeshiftComponent`) true)
    (else
      (bind _returnvalue (`KismetSystemLibrary.K2_SetTimerDelegate` (delegate `ExecOnUse`) 0.3))
      (set `self.DelayedExecTimer` _returnvalue))))

(fn `CanUseItem`
  (params (invokingCharacter :type "ConanCharacter Object Reference"))
  (returns (ReturnValue :type Boolean))
  (return true))