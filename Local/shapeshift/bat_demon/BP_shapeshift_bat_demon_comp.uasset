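; Shapeshift component that cycles a BaseBPChar from human into walking bat demon, toggles walking and flying, or restores human form on exit.
; ToggleForm swaps the main mesh's skeleton and anim class, hides all body meshes, and shows an added bat mesh slaved via master pose.
; Forms equip attack items looked up by name in ItemTable.
; Flight uses server-side CheatManager Fly/Walk, and character audio is muted while transformed.
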(event `ToggleFormEvent`
  (params (ExitShapeshift :type Boolean))
  (`self.ToggleForm` ExitShapeshift))

(fn `ToggleForm`
  (params (ExitShapeshift :type Boolean))
  (bind _returnvalue (`KismetMathLibrary.Conv_VectorToTransform` (0.0 0.0 0.0)))
  (bind _shapeshiftmesh (`self.ShapeshiftMesh`))
  (bind _mainmeshcomp (`self.MainMeshComp`))
  (bind _equipmentinventory (`/Game/Characters/BaseBPChar.EquipmentInventory` (`self.TargetCharacter`)))
  (bind _asbase_bpchar (cast `/Game/Characters/BaseBPChar` (`self.GetOwner`)))
  (set `self.TargetCharacter` _asbase_bpchar)
  (`|ExecutionSequence`
    (:`then_0`
      ;[1 1 1] One-time lookups
      (`/Game/Systems/BP_MacroGlobal.IsValid+Branch` (`self.MainMeshComp`) true
        (:`False or Invalid`
          (bind _ismale (`self.IsMale`)
            (:`ExecOut`
              (bind _matchingmeshcomp (`self.ForEachSKMesh` (select `bool` _ismale :`false` "SK_human_female" :`true` "SK_human_male"))
                (:`ExecMatch`
                  (bind _output_get (set `self.MainMeshComp` _matchingmeshcomp))
                  (set `self.OriginalSkelMesh` (`SkinnedMeshComponent.SkeletalMesh` _output_get))
                  (set `self.OriginalAnimClass` (`SkeletalMeshComponent.AnimClass` _output_get)))))))))
    (:`then_1`
      (if (== (`self.BatFormWeaponID`) 0)
        (bind _itemid (`self.FindItemByName` "BatDemonAttack")
          (:`ExecOut`
            (set `self.BatFormWeaponID` _itemid)))))
    (:`then_2`
      (if (== (`self.BatFormFlyingWeaponID`) 0)
        (bind _itemid_2 (`self.FindItemByName` "BatDemonFlyingAttack")
          (:`ExecOut`
            (set `self.BatFormFlyingWeaponID` _itemid_2)))))
    (:`then_3`
      (if ExitShapeshift
        (if (`self.IsShapeshifted`)
          ;[1 1 1] GoTo State Human
          (`self.SetSkinnedAssetAndUpdate` (`self.MainMeshComp`) (`self.OriginalSkelMesh`) true)
          (`self.SetAnimInstanceClass` (`self.MainMeshComp`) (`self.OriginalAnimClass`))
          (bind _matchingmeshcomp_2 (`self.ForEachSKMesh` "*")
            (:`ExecMatch`
              (`self.SetVisibility` _matchingmeshcomp_2 true false))
            (:`Complete`
              (`self.SetVisibility` (`self.MainMeshComp`) false false)
              (`self.SetVisibility` (`self.ShapeshiftMesh`) false false)
              (`self.ToggleFly` false
                (:`ExecOut`
                  (`self.ToggleSound` true
                    (:`ExecOut`
                      (set `self.IsShapeshifted` false)
                      (set `self.IsFlying` false)
                      (`ItemInventory.DeleteItems` _equipmentinventory (`ItemInventory.FindItemByTemplateID` _equipmentinventory (`self.BatFormWeaponID`) 0) 1)
                      (`ItemInventory.DeleteItems` _equipmentinventory (`ItemInventory.FindItemByTemplateID` _equipmentinventory (`self.BatFormFlyingWeaponID`) 0) 1))))))))
        (elif (`self.IsShapeshifted`)
          (if (`self.IsFlying`)
            ;[1 1 1] GoTo State Bat Demon (walking)
            (`self.SetSkinnedAssetAndUpdate` (`self.MainMeshComp`) "/Game/Characters/NPCs/Bat_Demon/Meshes/SK_bat_demon.SK_bat_demon" true :!label _label)
            (`self.SetAnimInstanceClass` (`self.MainMeshComp`) "/Game/Characters/NPCs/Bat_Demon/Animations/AB_Bat_Demon.AB_Bat_Demon_C")
            (bind _matchingmeshcomp_3 (`self.ForEachSKMesh` "*")
              (:`ExecMatch`
                (`self.SetVisibility` _matchingmeshcomp_3 false false))
              (:`Complete`
                (`/Game/Systems/BP_MacroGlobal.IsValid+Branch` _shapeshiftmesh true
                  (:`True`
                    (`self.K2_SetRelativeTransform` _shapeshiftmesh _returnvalue false false)
                    (`self.SetVisibility` (`self.ShapeshiftMesh`) true false)
                    (`self.ToggleFly` false
                      (:`ExecOut`
                        _)))
                  (:`False or Invalid`
                    (bind _returnvalue_2 (`CharacterFunctionLibrary.AddSkeletalMeshComponent` (`self.TargetCharacter`) false _returnvalue "/Script/Engine.SkeletalMeshComponent"))
                    (bind _output_get_2 (set `self.ShapeshiftMesh` _returnvalue_2))
                    (`self.SetSkinnedAssetAndUpdate` _output_get_2 "/Game/Characters/NPCs/Bat_Demon/Meshes/SK_bat_demon.SK_bat_demon" true)
                    (`self.K2_AttachToComponent` _output_get_2 _mainmeshcomp "None" "KeepRelative" "KeepRelative" "KeepRelative" true)
                    (`self.SetLeaderPoseComponent` _output_get_2 _mainmeshcomp)))
                (`self.ToggleSound` false
                  (:`ExecOut`
                    (bind _returnvalue_3 (`GameItemSpawner.SpawnItem` "GameItem" (`self.BatFormWeaponID`)))
                    (`EquipmentInventory.AddItemToSlot` (`/Game/Characters/BaseBPChar.EquipmentInventory` (`self.TargetCharacter`)) "DualHand" _returnvalue_3)
                    (set `self.IsShapeshifted` true)
                    (set `self.IsFlying` false)))))
            (else
              ;[1 1 1] GoTo State Bat Demon (flying)
              (`self.K2_SetRelativeTransform` (`self.ShapeshiftMesh`) (`KismetMathLibrary.Conv_VectorToTransform` (0.0 0.0 -300.0)) false false)
              (`self.SetAnimInstanceClass` (`self.MainMeshComp`) "/Game/Mods/ThraxersTestMod/shapeshift/bat_demon/animation/AB_Bat_Demon_Flying.AB_Bat_Demon_Flying_C")
              (set `CharacterMovementComponent.MaxFlySpeed` 1000.0 (`Character.CharacterMovement` (`self.TargetCharacter`)))
              (`self.ToggleFly` true
                (:`ExecOut`
                  (bind _returnvalue_4 (`GameItemSpawner.SpawnItem` "GameItem" (`self.BatFormFlyingWeaponID`)))
                  (`EquipmentInventory.AddItemToSlot` (`/Game/Characters/BaseBPChar.EquipmentInventory` (`self.TargetCharacter`)) "DualHand" _returnvalue_4)
                  (set `self.IsShapeshifted` true)
                  (set `self.IsFlying` true)))))
          (else
            (goto _label)))))))